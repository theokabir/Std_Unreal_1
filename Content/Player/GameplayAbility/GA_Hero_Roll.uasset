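; Gameplay ability for the hero's dodge roll, steered by the last movement input.
; After a brief delay, it feeds that direction to Motion Warping as a rotation target.
; It also projects a level-scaled distance along the direction, traces down for ground, and uses the impact point as the translation warp target.
; It then plays the roll montage, ending the ability when it completes, blends out or is interrupted or cancelled.
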(event `self.K2_ActivateAbility`
  (`KismetSystemLibrary.Delay` 0.05)
  (`self.CumputeRollDirectionAndDistance`)
  (`AbilityTask_PlayMontageAndWait.CreatePlayMontageAndWaitProxy` "None" "/Game/Player/Montages/AM_Hero_Roll.AM_Hero_Roll"
    (:`OnCompleted`
      _)
    (:`OnBlendOut`
      _)
    (:`OnInterrupted`
      _)
    (:`OnCancelled`
      _))
  (`self.K2_EndAbility`))

(fn `CumputeRollDirectionAndDistance`
  (locals (CachedRollingDirection :type "Vector Structure" :default (0.0 0.0 0.0)))
  (bind _returnvalue (`self.GetHeroCharacterFromActorInfo`))
  (bind _returnvalue_2 (+ (* (`local.CachedRollingDirection`) (`WarriorFunctionLibrary.GetScalableFloatValueAtLevel` (`self.Rolling Distance Scalable Float`) (`KismetMathLibrary.Conv_IntToDouble` (`self.GetAbilityLevel`)))) (`Actor.K2_GetActorLocation` _returnvalue)))
  (set `local.CachedRollingDirection` (`KismetMathLibrary.Normal` (`Pawn.GetLastMovementInputVector` (`self.GetHeroCharacterFromActorInfo`))))
  (`|ExecutionSequence`
    (:`then_0`
      ;[0.03394 0.15 0.06612 0.5] Execute Rotation Motion Warp
      (`MotionWarpingComponent.AddOrUpdateWarpTargetFromLocationAndRotation` (`WarriorBaseCharacter.WarpingComponent` (`self.GetHeroCharacterFromActorInfo`)) "RollingDirection" (0.0 0.0 0.0) (`KismetMathLibrary.MakeRotFromX` (`local.CachedRollingDirection`))))
    (:`then_1`
      ;[0.15 0.05859 0.05859 0.5] Execute Translation Motion Warop On Destiny
      (bind _outhit (`KismetSystemLibrary.LineTraceSingleForObjects` _returnvalue_2 (+ _returnvalue_2 (* (`Actor.GetActorUpVector` _returnvalue) -600.0)) (`self.Object Types`)))
      (`MotionWarpingComponent.AddOrUpdateWarpTargetFromLocation` (`WarriorBaseCharacter.WarpingComponent` (`self.GetHeroCharacterFromActorInfo`)) "RollTargetLocation" (`.ImpactPoint` (`GameplayStatics.BreakHitResult` _outhit))))))