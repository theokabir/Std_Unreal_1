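; Base enemy character Blueprint that plays a dissolve death sequence when the enemy dies.
; On death it pauses animation, disables capsule collision and async-loads a Niagara system attached to the mesh, tinted from the material's dissolve edge color.
; A timeline scaled to the total dissolve time drives the dissolve parameter on body and equipped weapon materials, then destroys both actors.
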(event `/Game/EnemyCharacter/BPI_EnemyDeath.OnEnemyDied`
  (params (DissolveNiagraSystem :type "NiagaraSystem Soft Object Reference"))
  (bind _mesh (`self.Mesh`))
  (bind _returnvalue (`PawnCombatComponent.GetCurrentEquippedWeapon` (`self.EnemyCombatComponent`)))
  (bind _returnvalue_2 (`PawnCombatComponent.GetCurrentEquippedWeapon` (`self.EnemyCombatComponent`)))
  (`|ExecutionSequence`
    (:`then_0`
      ;[0.02796 0.15 0.06904 0.5] Disable collision
      (set `SkeletalMeshComponent.bPauseAnims` true (`self.Mesh`))
      (`PrimitiveComponent.SetCollisionEnabled` (`self.CapsuleComponent`) "NoCollision"))
    (:`then_1`
      ;[0.01313 0.1075 0.15 0.5] Spawn Niagara Particles
      (bind _object (`|LoadAsset` DissolveNiagraSystem)
        (:`Completed`
          (bind _asniagara_system (cast `NiagaraSystem` _object))
          (bind _returnvalue_3 (`NiagaraFunctionLibrary.SpawnSystemAttached` _asniagara_system (`self.Mesh`) "None" (0.0 0.0 0.0) (struct) "KeepRelativeOffset" true))
          (bind _returnvalue_4 (`PrimitiveComponent.CreateDynamicMaterialInstance` _mesh 0 (`PrimitiveComponent.GetMaterial` _mesh 0) "None"))
          (bind _returnvalue_5 (`MaterialInstanceDynamic.K2_GetVectorParameterValue` _returnvalue_4 "DissolveEdgeColor"))
          (`NiagaraComponent.SetNiagaraVariableLinearColor` _returnvalue_3 "DissolveParticleColor" _returnvalue_5))))
    (:`then_2`
      ;[0.15 0.02031 0.02031 0.5] Dissolve Material
      (`TimelineComponent.SetPlayRate` (`self.Timeline`) (/ 1.0 (`self.Total Dissolved Time`)))
      (bind (_direction _normalizedfloattrack) (`Timeline|Timeline` :!via `PlayFromStart`)
        (:`Update`
          (`MeshComponent.SetScalarParameterValueOnMaterials` (`self.Mesh`) "DissolveAmount" _normalizedfloattrack)
          (`/Engine/EditorBlueprintResources/StandardMacros.IsValid` _returnvalue_2
            (:`Is Valid`
              (`MeshComponent.SetScalarParameterValueOnMaterials` (`WarriorWeaponBase.WeaponMesh` _returnvalue_2) "DissolveAmount" _normalizedfloattrack))))
        (:`Finished`
          (`/Engine/EditorBlueprintResources/StandardMacros.IsValid` _returnvalue
            (:`Is Valid`
              (`self.K2_DestroyActor` _returnvalue))
            (:`Is Not Valid`
              _))
          (`self.K2_DestroyActor`))))))

(fn `UserConstructionScript`)